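; Openable door actor that swings open and closed in response to open and close requests from its OpenDoor component.
; A timeline plays forward to open and in reverse to close, adding its OpenAngle curve as yaw to the rotation cached at BeginPlay.
; An event track on the same timeline times the door lock sound played at the actor's location.
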(event `self.ReceiveBeginPlay`
  (set `self.InitialRotation` (`self.K2_GetActorRotation`)))

(event `self.OpenDoor.OnOpenRequest`
  (bind (_direction _open_angle) (`Timeline|DoorSwing_Timeline` :!label _label)
    (:`Update`
      (`self.K2_SetActorRotation` (`KismetMathLibrary.ComposeRotators` (`self.InitialRotation`) (`KismetMathLibrary.MakeRotator` 0.0 0.0 _open_angle))))
    (:`Sound Timing`
      (`GameplayStatics.PlaySoundAtLocation` "/Game/Audio/door-lock.door-lock" (`self.K2_GetActorLocation`) (struct) 1.0 1.0 0.0 null null null))))

(event `self.OpenDoor.OnCloseRequest`
  (goto _label :!via `Reverse`))

(fn `UserConstructionScript`)